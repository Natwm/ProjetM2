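; Example save actor that stores and restores the PlayerRunner's position, best time and checkpoint best time in a single save slot.
; BeginPlay creates a fresh SaveGameData object and immediately saves over the slot without loading it first.
; T saves and L loads, teleporting the player, zeroing JumpPoint and calling the runner's best-time reset and reload events.
; An automatic load of the last save is left unconnected.
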(event `self.ReceiveBeginPlay`
  ;[1 1 1] Create save game object
  (bind _returnvalue (`GameplayStatics.CreateSaveGameObject` "/Game/BluePrint/SaveData/SaveGameData.SaveGameData_C"))
  (set `self.SaveGameDataRef` _returnvalue)
  (`self.Save Data`))

(event `Load Save File`
  (bind _savegamedataref (`self.SaveGameDataRef`))
  ;[1 1 1] Load save file
  (bind _returnvalue (`GameplayStatics.LoadGameFromSlot` "MySaveGame"))
  (bind _assave_game_data (cast `/Game/BluePrint/SaveData/SaveGameData` _returnvalue))
  (set `self.SaveGameDataRef` _assave_game_data)
  (bind _asplayer_runner (cast `/Game/BluePrint/Player/PlayerRunner` (`GameplayStatics.GetPlayerPawn` 0)))
  (set `/Game/BluePrint/Player/PlayerRunner.Player_BestTime` (`/Game/BluePrint/SaveData/SaveGameData.BestTime` (`self.SaveGameDataRef`)) _asplayer_runner)
  ;[1 1 1] Set Load Data
  (`self.K2_SetActorLocation` _asplayer_runner (`/Game/BluePrint/SaveData/SaveGameData.PlayerPos` _savegamedataref) false true)
  (set `/Game/BluePrint/Player/PlayerRunner.Player_BestCheckPointTime` (`/Game/BluePrint/SaveData/SaveGameData.BestTime_CheckPoint_1` _savegamedataref) _asplayer_runner)
  (set `/Game/BluePrint/Player/PlayerRunner.Player_BestTime` (`/Game/BluePrint/SaveData/SaveGameData.BestTime` _savegamedataref) _asplayer_runner)
  (bind _asplayer_runner_2 (cast `/Game/BluePrint/Player/PlayerRunner` (`GameplayStatics.GetPlayerPawn` 0)))
  (set `/Game/BluePrint/Player/PlayerRunner.Jump Point` 0 _asplayer_runner_2)
  (`/Game/BluePrint/Player/PlayerRunner.ResetBestTime` _asplayer_runner_2)
  (`/Game/BluePrint/Player/PlayerRunner.Reload` _asplayer_runner_2))

(event `Save Data`
  (bind _savegamedataref (`self.SaveGameDataRef`))
  ;[1 1 1] Save data
  (bind _asplayer_runner (cast `/Game/BluePrint/Player/PlayerRunner` (`GameplayStatics.GetPlayerPawn` 0)))
  (set `/Game/BluePrint/SaveData/SaveGameData.BestTime` (`/Game/BluePrint/Player/PlayerRunner.Player_BestTime` _asplayer_runner) _savegamedataref)
  (set `/Game/BluePrint/SaveData/SaveGameData.BestTime_CheckPoint_1` (`/Game/BluePrint/Player/PlayerRunner.Player_BestCheckPointTime` _asplayer_runner) _savegamedataref)
  (set `/Game/BluePrint/SaveData/SaveGameData.PlayerPos` (`self.K2_GetActorLocation` (`GameplayStatics.GetPlayerPawn` 0)) _savegamedataref)
  ;[1 1 1] Save to file
  (`GameplayStatics.SaveGameToSlot` (`self.SaveGameDataRef`) "MySaveGame")
  (`KismetSystemLibrary.PrintText` "Game Saved"))

(event `Key|T`
  (params (Key :type "Key Structure"))
  (:`Pressed`
    (`self.Save Data`)))

(event `Key|L`
  (params (Key :type "Key Structure"))
  (:`Pressed`
    (`self.Load Save File`)))

(fn `UserConstructionScript`)