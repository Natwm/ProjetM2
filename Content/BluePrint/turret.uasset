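; Rotating turret obstacle with two cubes that raise or lower a PlayerRunner's jump points on overlap.
; On BeginPlay, each Conponents flag picks a cube's material from MatA, while PlatformTag is assigned as its tags in either case.
; Tick yaws the root by Speed each frame.
; On overlap, a cube whose first tag is "Trigger+" adds a jump point; otherwise it subtracts one.
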(event `self.ReceiveBeginPlay`
  (bind _cube_2 (`self.Cube 2`))
  (bind _cube_1 (`self.Cube 1`))
  (bind _cube_1_2 (`self.Cube 1`))
  (bind _cube_2_2 (`self.Cube 2`))
  (for _index (range (`KismetArrayLibrary.Array_Length` (`self.Conponents`)))
    (if (== _index 0)
      (bind _output (`|GetArrayItem` (`self.Conponents`) _index))
      (if _output
        (`PrimitiveComponent.SetMaterial` _cube_1 0 (`|GetArrayItem` (`self.MatA`)))
        (set `ActorComponent.ComponentTags` (`self.Platform Tag +`) _cube_1)
        (else
          (`PrimitiveComponent.SetMaterial` _cube_1_2 0 (`|GetArrayItem` (`self.MatA`) 1))
          (set `ActorComponent.ComponentTags` (`self.Platform Tag -`) _cube_1_2)))
      (elif _output
        (`PrimitiveComponent.SetMaterial` _cube_2_2 0 (`|GetArrayItem` (`self.MatA`)))
        (set `ActorComponent.ComponentTags` (`self.Platform Tag +`) _cube_2_2)
        (else
          (`PrimitiveComponent.SetMaterial` _cube_2 0 (`|GetArrayItem` (`self.MatA`) 1))
          (set `ActorComponent.ComponentTags` (`self.Platform Tag -`) _cube_2))))))

(event `self.ReceiveTick`
  (params (DeltaSeconds :type "Float (single-precision)"))
  (`SceneComponent.K2_AddRelativeRotation` (`self.DefaultSceneRoot`) (`KismetMathLibrary.MakeRotator` 0.0 0.0 (`self.Speed`)) false false))

(event `self.Cube 1.OnComponentBeginOverlap`
  (params (OverlappedComponent :type "PrimitiveComponent Object Reference") (OtherActor :type "Actor Object Reference") (OtherComp :type "PrimitiveComponent Object Reference") (OtherBodyIndex :type Integer) (bFromSweep :type Boolean) (SweepResult :type "HitResult Structure (by ref)"))
  (bind _asplayer_runner (cast `/Game/BluePrint/Player/PlayerRunner` OtherActor))
  (if (`KismetStringLibrary.EqualEqual_StrStr` (`KismetStringLibrary.Conv_NameToString` (`|GetArrayItem` (`ActorComponent.ComponentTags` (`self.Cube 1`)))) "Trigger+")
    (`/Game/BluePrint/Player/PlayerRunner.AddJumpPoint` _asplayer_runner 1)
    (else
      (`/Game/BluePrint/Player/PlayerRunner.AddJumpPoint` _asplayer_runner -1))))

(event `self.Cube 2.OnComponentBeginOverlap`
  (params (OverlappedComponent :type "PrimitiveComponent Object Reference") (OtherActor :type "Actor Object Reference") (OtherComp :type "PrimitiveComponent Object Reference") (OtherBodyIndex :type Integer) (bFromSweep :type Boolean) (SweepResult :type "HitResult Structure (by ref)"))
  (bind _asplayer_runner (cast `/Game/BluePrint/Player/PlayerRunner` OtherActor))
  (if (`KismetStringLibrary.EqualEqual_StrStr` (`KismetStringLibrary.Conv_NameToString` (`|GetArrayItem` (`ActorComponent.ComponentTags` (`self.Cube 2`)))) "Trigger+")
    (`/Game/BluePrint/Player/PlayerRunner.AddJumpPoint` _asplayer_runner 1)
    (else
      (`/Game/BluePrint/Player/PlayerRunner.AddJumpPoint` _asplayer_runner -1))))

(fn `UserConstructionScript`)