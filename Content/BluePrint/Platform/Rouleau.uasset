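; Rouleau is a roller platform actor that spins its Cylinder component continuously.
; Each tick it adds Speed to the cylinder's relative yaw, without scaling by delta time, so the spin rate depends on frame rate.
; An unconnected timeline that would move the cylinder along a Spline never runs, and its Reverse event is empty.
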(event `self.ReceiveTick`
  (params (DeltaSeconds :type "Float (single-precision)"))
  (`SceneComponent.K2_AddRelativeRotation` (`self.Cylinder`) (`KismetMathLibrary.MakeRotator` 0.0 0.0 (`self.Speed`)) false false))

(event `self.ReceiveBeginPlay`)

(event `Reverse`)

(fn `UserConstructionScript`)