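; Checkpoint actor for a runner game that reacts once when a player-tagged PlayerRunner overlaps its Trigger.
; A non-negative Index notifies the runner of that checkpoint and saves the checkpoint's rotation through the first GameSaverExample actor found in the level.
; A negative Index makes it the finish line, ending the run.
; Either path then destroys the Trigger; the feedback audio playback is left unconnected.
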(event `self.Trigger.OnComponentBeginOverlap`
  (params (OverlappedComponent :type "PrimitiveComponent Object Reference") (OtherActor :type "Actor Object Reference") (OtherComp :type "PrimitiveComponent Object Reference") (OtherBodyIndex :type Integer) (bFromSweep :type Boolean) (SweepResult :type "HitResult Structure (by ref)"))
  (if (`self.ActorHasTag` OtherActor "Player")
    (bind _asplayer_runner (cast `/Game/BluePrint/Player/PlayerRunner` OtherActor))
    (if (>= (`self.Index`) 0)
      (`/Game/BluePrint/Player/PlayerRunner.OnCheckPointCollapse` _asplayer_runner (`self.Index`))
      (bind _outactors (`GameplayStatics.GetAllActorsOfClass` "/Game/BluePrint/SaveData/GameSaverExample.GameSaverExample_C"))
      (`/Game/BluePrint/SaveData/GameSaverExample.Save Data` (`|GetArrayItem` _outactors) (`self.K2_GetActorRotation`))
      (else
        (`/Game/BluePrint/Player/PlayerRunner.OnFinishRun` _asplayer_runner)))
    (`ActorComponent.K2_DestroyComponent` (`self.Trigger`))))

(fn `UserConstructionScript`)