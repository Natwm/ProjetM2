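; A scaling platform Blueprint that, after a random delay, endlessly grows and shrinks along one selectable axis.
; Tick counts down a time picked between MinTime and MaxTime, then starts the timeline once.
; Each timeline update adds an increment to the actor's current scale, weighted by the PlatformDistance curve and MultiplicatorScale, rather than interpolating between fixed sizes.
; On finish, Reverse flips the increment's sign and alternates timeline playback direction.
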(event `PlayScale`
  (bind (_direction _platform_distance) (`Timeline|Timeline_1` :!label _label)
    (:`Update`
      (if (`self.Is Reverse`)
        (switch `/Game/ScalePlatform` (`self.ScaleDirection`)
          (:`NewEnumerator0`
            (set `self.ScaleX` (-0.1 0.0 0.0)))
          (:`NewEnumerator1`
            (set `self.ScaleX` (0.0 -0.1 0.0)))
          (:`NewEnumerator2`
            (set `self.ScaleX` (0.0 0.0 -0.1))))
        (else
          (switch `/Game/ScalePlatform` (`self.ScaleDirection`)
            (:`NewEnumerator0`
              (set `self.ScaleX` (0.1 0.0 0.0)))
            (:`NewEnumerator1`
              (set `self.ScaleX` (0.0 0.1 0.0)))
            (:`NewEnumerator2`
              (set `self.ScaleX` (0.0 0.0 0.1))))))
      (`self.SetActorScale3D` (+ (* (* (`self.ScaleX`) _platform_distance) (`self.multiplicator Scale`)) (`self.GetActorScale3D`))))
    (:`Finished`
      (`self.Reverse`))))

(event `self.ReceiveTick`
  (params (DeltaSeconds :type "Float (single-precision)"))
  (if (not (`self.test`))
    (if (== (`self.Time`) 0.0)
      (bind _output_get (set `self.Time` (`KismetMathLibrary.RandomFloatInRange` (`self.MinTime`) (`self.MaxTime`)))))
    (set `self.Time` (- _output_get DeltaSeconds))
    (if (<= (`self.Time`) 0.0)
      (set `self.test` true)
      (`self.PlayScale`)
      (else
        (set `self.test` false)))))

(event `Reverse`
  (if (`self.Is Reverse`)
    (set `self.Is Reverse` false)
    (goto _label :!via `PlayFromStart`)
    (else
      (set `self.Is Reverse` true)
      (goto _label :!via `Reverse`))))

(fn `UserConstructionScript`)