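; Bumper platform actor that launches the player along a configurable launch vector scaled by bumper power.
; When a Player-tagged PlayerTest enters its box, it cuts the character's velocity to a third, then adds the launch through LaunchCharacter without overriding existing velocity.
; On BeginPlay it draws a long-lived debug arrow showing launch direction and scaled strength, and prints the vector's components on a text render.
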(event `self.ReceiveBeginPlay`
  (bind (_launch_vector_x _launch_vector_y _launch_vector_z) (`KismetMathLibrary.BreakVector` (`self.Launch Vector`)))
  (bind _returnvalue (+ (`self.K2_GetActorLocation`) (0.0 0.0 50.0)))
  ;[0.2542 0.1912 0.04971] Start
  (`KismetSystemLibrary.DrawDebugArrow` _returnvalue (+ _returnvalue (* (`self.Launch Vector`) (/ (`self.Bumper power`) 2.5))) 200.0 (struct :`R` 1.0 :`A` 1.0) 500.0 3.0)
  (`TextRenderComponent.K2_SetText` (`self.TextRender`) (`KismetTextLibrary.Conv_StringToText` (`KismetStringLibrary.Concat_StrStr` (`KismetStringLibrary.Conv_DoubleToString` _launch_vector_x) (`KismetStringLibrary.Conv_DoubleToString` _launch_vector_y) (`KismetStringLibrary.Conv_DoubleToString` _launch_vector_z)))))

(event `self.Box.OnComponentBeginOverlap`
  (params (OverlappedComponent :type "PrimitiveComponent Object Reference") (OtherActor :type "Actor Object Reference") (OtherComp :type "PrimitiveComponent Object Reference") (OtherBodyIndex :type Integer) (bFromSweep :type Boolean) (SweepResult :type "HitResult Structure (by ref)"))
  ;[0.2961 0.01521 0.01521] Bumper
  ;;[0.02624 0.162 0.1714] Check If Player
  (if (`self.ActorHasTag` OtherActor "Player")
    (bind _asplayer_test (cast `/Game/BluePrint/Player/PlayerTest` OtherActor))
    ;;[0.05286 0.2307 0.3663] Reset Velocity before propulse
    (set `MovementComponent.Velocity` (/ (`self.GetVelocity` _asplayer_test) 3.0) (`Character.CharacterMovement` _asplayer_test))
    (`Character.LaunchCharacter` _asplayer_test (* (`self.Launch Vector`) (`self.Bumper power`)) false false)))

(fn `UserConstructionScript`)